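; BP_Potion is a colored, lockable item that passes its color to any BP_ColoredBlock that begins overlapping its Collision component.
; The construction script creates a dynamic M_Potion material on the Item component and tints its Base Color to match.
; UnlockItem calls the parent version, then clears the constraint mode on Item.
; LockItem resets Item's world rotation and restores the default constraint mode, without calling the parent.
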(event `self.Collision.OnComponentBeginOverlap`
  (params (OverlappedComponent :type "PrimitiveComponent Object Reference") (OtherActor :type "Actor Object Reference") (OtherComp :type "PrimitiveComponent Object Reference") (OtherBodyIndex :type Integer) (bFromSweep :type Boolean) (SweepResult :type "HitResult Structure (by ref)"))
  (bind _asbp_colored_block (cast `/Game/Blueprints/BP_ColoredBlock` OtherActor))
  (`/Game/Blueprints/BP_ColoredBlock.SetColor` _asbp_colored_block (`self.Color`)))

(fn `LockItem`
  (bind _item (`self.Item`))
  (`SceneComponent.K2_SetWorldRotation` :`self` _item)
  (`PrimitiveComponent.SetConstraintMode` _item "Default"))

(fn `UnlockItem`
  (`parent.UnlockItem`)
  (`PrimitiveComponent.SetConstraintMode` (`self.Item`) "None"))

(fn `UserConstructionScript`
  (bind _returnvalue (`PrimitiveComponent.CreateDynamicMaterialInstance` (`self.Item`) 0 "/Game/Materials/M_Potion.M_Potion" "None"))
  (`MaterialInstanceDynamic.SetVectorParameterValue` _returnvalue "Base Color" (`KismetMathLibrary.Conv_ColorToLinearColor` (`self.Color`))))