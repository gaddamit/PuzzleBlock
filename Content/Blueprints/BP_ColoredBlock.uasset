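; Colored block item that takes on the color of any BP_Potion that begins overlapping it.
; SetColor puts a dynamic M_Solid material instance on the mesh, sets its Base Color and stores the color.
; UnlockItem extends the parent by clearing the constraint mode, disabling pad overlap events and switching to physics-only collision.
; LockItem re-enables pad overlaps and query collision, and zeroes rotation, without calling the parent.
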(event `self.Item.OnComponentBeginOverlap`
  (params (OverlappedComponent :type "PrimitiveComponent Object Reference") (OtherActor :type "Actor Object Reference") (OtherComp :type "PrimitiveComponent Object Reference") (OtherBodyIndex :type Integer) (bFromSweep :type Boolean) (SweepResult :type "HitResult Structure (by ref)"))
  (bind _asbp_potion (cast `/Game/Blueprints/BP_Potion` OtherActor))
  (`self.SetColor` (`/Game/Blueprints/BP_CarryableItem.Color` _asbp_potion)))

(fn `LockItem`
  (set `PrimitiveComponent.bGenerateOverlapEvents` true (`self.CollisionForpad`))
  (`PrimitiveComponent.SetCollisionEnabled` (`self.Item`) "QueryAndPhysics")
  (`SceneComponent.K2_SetWorldRotation` :`self` (`self.Item`)))

(fn `SetColor`
  (params (Color :type "Color Structure"))
  (bind _returnvalue (`KismetMathLibrary.Conv_ColorToLinearColor` Color))
  (bind _returnvalue_2 (`PrimitiveComponent.CreateDynamicMaterialInstance` (`self.Item`) 0 "/Game/LevelPrototyping/Materials/M_Solid.M_Solid" "None"))
  (`MaterialInstanceDynamic.SetVectorParameterValue` _returnvalue_2 "Base Color" _returnvalue)
  (set `self.Color` (`KismetMathLibrary.Conv_LinearColorToColor` _returnvalue)))

(fn `UnlockItem`
  (`parent.UnlockItem`)
  (`PrimitiveComponent.SetConstraintMode` (`self.Item`) "None")
  (set `PrimitiveComponent.bGenerateOverlapEvents` false (`self.CollisionForpad`))
  (`PrimitiveComponent.SetCollisionEnabled` (`self.Item`) "PhysicsOnly"))

(fn `UserConstructionScript`
  (`parent.UserConstructionScript`))