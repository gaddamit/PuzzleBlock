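; BP_CarryableItem is a colored item actor that can be carried and dropped, tracked by an IsBeingCarried flag.
; The construction script applies a dynamic M_Solid material to Item, tinted with the Color variable.
; CarryItem raises Item by CarryHeight and calls UnlockItem, while DropItem clears the flag and calls LockItem without lowering it.
; LockItem and UnlockItem are empty here, and the event graph has no active logic.
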(fn `CarryItem`
  (set `self.IsBeingCarried` true)
  (`SceneComponent.K2_AddWorldOffset` (`self.Item`) (`KismetMathLibrary.MakeVector` 0.0 0.0 (`self.CarryHeight`)) false false)
  (`self.UnlockItem`))

(fn `DropItem`
  (set `self.IsBeingCarried` false)
  (`self.LockItem`))

(fn `LockItem`)

(fn `UnlockItem`)

(fn `UserConstructionScript`
  (bind _returnvalue (`PrimitiveComponent.CreateDynamicMaterialInstance` (`self.Item`) 0 "/Game/LevelPrototyping/Materials/M_Solid.M_Solid" "None"))
  (`MaterialInstanceDynamic.SetVectorParameterValue` _returnvalue "Base Color" (`KismetMathLibrary.Conv_ColorToLinearColor` (`self.Color`))))